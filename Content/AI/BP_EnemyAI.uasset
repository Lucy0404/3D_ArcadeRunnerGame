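; Enemy pawn that chases the player on sight and triggers the defeat screen on catching them.
; PawnSensing's OnSeePawn sets a seen flag, without checking which pawn was seen, and starts an AI MoveTo toward the player character.
; When the move succeeds, it plays a defeat sound, shows and animates the WB_Defeat widget, switches to UI-only input with a cursor and pauses the game.
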(event `self.ReceiveTick`
  (params (DeltaSeconds :type "Float (single-precision)")))

(event `self.PawnSensing.OnSeePawn`
  (params (Pawn :type "Pawn Object Reference"))
  (set `self.IsSeeingPlayer?` true)
  (`self.FollowPlayer`))

(event `FollowPlayer`
  (bind _returnvalue (`GameplayStatics.GetPlayerController` 0))
  (if (`self.IsSeeingPlayer?`)
    (`|AIMoveTo` self (0.0 0.0 0.0) (`GameplayStatics.GetPlayerCharacter` 0) 70.0
      (:`OnSuccess`
        (`GameplayStatics.PlaySound2D` "/Game/Music/DefeatSound.DefeatSound" 1.0 1.0 0.0 null null)
        (bind _returnvalue_2 (`|CreateWidget` "/Game/UI/WB_Defeat.WB_Defeat_C"))
        (`UserWidget.AddToViewport` _returnvalue_2 0)
        (set `PlayerController.bShowMouseCursor` true _returnvalue)
        (`WidgetBlueprintLibrary.SetInputMode_UIOnlyEx` _returnvalue null)
        (`/Game/UI/WB_Defeat.DefeatAnim` _returnvalue_2)
        (`GameplayStatics.SetGamePaused` true)))))

(fn `UserConstructionScript`)